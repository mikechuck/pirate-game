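; Blunderbuss weapon Blueprint for BoatFight that fires bullets when used.
; UseWeapon calls the parent implementation, then spawns a BP_Bullet at the BulletSpawn component's world transform, regardless of collision.
; BeginPlay, Shoot and the item action event only print debug strings, and the code binding that event to BP_Character is disconnected.
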(event `self.ReceiveBeginPlay`
  (`KismetSystemLibrary.PrintString` "Hello"))

(event `ItemAction_Event_0`
  (`KismetSystemLibrary.PrintString` "Hello"))

(fn `Shoot`
  (`KismetSystemLibrary.PrintString` "Shooting"))

(fn `UserConstructionScript`)

(fn `UseWeapon`
  (`parent.UseWeapon`)
  ;[1 1 1] Shoot bullet from BulletSpawn component
  (bind _asscene_component (cast `SceneComponent` (`self.BulletSpawn`)))
  (`|SpawnActorFromClass` "/Game/BoatFight/Blueprints/Projectiles/BP_Bullet.BP_Bullet_C" (`SceneComponent.K2_GetComponentToWorld` _asscene_component) "AlwaysSpawn" "MultiplyWithRoot" null null))