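; BP_Cannon is a possessable cannon that the player aims, fires and exits through Enhanced Input.
; On controller change it swaps input to the cannon mapping context.
; Look input yaws the root and rolls the barrel, trimming each delta to clamp against the BeginPlay rotation without stutter.
; Shooting spawns BP_Cannonball at CannonballSpawn; exiting detaches the stored character, restores collision and mobility, and repossesses it.
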(event `self.ReceiveBeginPlay`
  (set `self.StartingRotation` (`SceneComponent.K2_GetComponentRotation` (`self.DefaultSceneRoot`))))

(event `EnhancedInput|/Game/BoatFight/Inputs/Cannon/IA_Cannon_Look`
  (params (ActionValue :type "Vector2D Structure") (ElapsedSeconds :type "Float (double-precision)") (TriggeredSeconds :type "Float (double-precision)") (InputAction :type "InputAction Object Reference" :default "/Game/BoatFight/Inputs/Cannon/IA_Cannon_Look.IA_Cannon_Look"))
  ;[1 1 1] Cannon controls
  ;;[1 1 1] Cannon camera input
  (:`Triggered`
    (`self.TurnCannon` ActionValue_X ActionValue_Y)))

(event `self.ReceiveControllerChanged`
  (params (OldController :type "Controller Object Reference") (NewController :type "Controller Object Reference"))
  (`self.BindControls`))

(event `EnhancedInput|/Game/BoatFight/Inputs/Cannon/IA_Cannon_Interact`
  (params (ActionValue :type Boolean) (ElapsedSeconds :type "Float (double-precision)") (TriggeredSeconds :type "Float (double-precision)") (InputAction :type "InputAction Object Reference" :default "/Game/BoatFight/Inputs/Cannon/IA_Cannon_Interact.IA_Cannon_Interact"))
  ;[1 1 1] Cannon controls
  ;;[1 1 1] Exit cannon input
  (:`Triggered`
    (`self.ExitCannon`)))

(event `self.ReceiveTick`
  (params (DeltaSeconds :type "Float (single-precision)")))

(event `EnhancedInput|/Game/BoatFight/Inputs/Cannon/IA_Cannon_Shoot`
  (params (ActionValue :type Boolean) (ElapsedSeconds :type "Float (double-precision)") (TriggeredSeconds :type "Float (double-precision)") (InputAction :type "InputAction Object Reference" :default "/Game/BoatFight/Inputs/Cannon/IA_Cannon_Shoot.IA_Cannon_Shoot"))
  ;[1 1 1] Cannon controls
  (:`Triggered`
    (`self.ShootCannon`)))

(fn `BindControls`
  ;[1 1 1] Add cannon mapping context
  (bind _asplayer_controller (cast `PlayerController` (`self.GetController`)))
  (bind _returnvalue (pcsubsystem `EnhancedInputLocalPlayerSubsystem` _asplayer_controller))
  (`EnhancedInputSubsystemInterface.ClearAllMappings` _returnvalue)
  (`EnhancedInputSubsystemInterface.AddMappingContext` _returnvalue "/Game/BoatFight/Inputs/Cannon/IMC_Cannon.IMC_Cannon" 0 (struct)))

(fn `ExitCannon`
  (bind _playercharacterpawn (`self.PlayerCharacterPawn`))
  ;[1 1 1] Detach player from boat
  (`self.K2_DetachFromActor` _playercharacterpawn "KeepWorld" "KeepWorld" "KeepWorld")
  ;[1 1 1] Allow player to move again
  (`self.SetActorEnableCollision` _playercharacterpawn true)
  (`SceneComponent.SetMobility` (`Actor.RootComponent` _playercharacterpawn) "Movable")
  ;[1 1 1] Possess player
  (bind _asbp_character (cast `/Game/BoatFight/Blueprints/BP_Character` _playercharacterpawn))
  (`Controller.Possess` (`PlayerState.GetPlayerController` (`GameplayStatics.GetPlayerState` 0)) _asbp_character))

(fn `ShootCannon`
  ;[1 1 1] Shoot bullet from BulletSpawn component
  (bind _asscene_component (cast `SceneComponent` (`self.CannonballSpawn`)))
  (`|SpawnActorFromClass` "/Game/BoatFight/Blueprints/Projectiles/BP_Cannonball.BP_Cannonball_C" (`SceneComponent.K2_GetComponentToWorld` _asscene_component) "AlwaysSpawn" "MultiplyWithRoot" null null))

(fn `TurnCannon`
  (params (TurnX :type "Float (double-precision)") (TurnY :type "Float (double-precision)"))
  (locals (TurnXValue :type "Float (double-precision)") (TurnYValue :type "Float (double-precision)"))
  (bind _startingrotation_roll (`KismetMathLibrary.BreakRotator` (`self.StartingRotation`)))
  (bind (_startingrotation_roll_2 _startingrotation_pitch _startingrotation_yaw) (`KismetMathLibrary.BreakRotator` (`self.StartingRotation`)))
  (bind (_returnvalue_roll _returnvalue_pitch _returnvalue_yaw) (`KismetMathLibrary.BreakRotator` (`SceneComponent.K2_GetComponentRotation` (`self.DefaultSceneRoot`))))
  (bind _returnvalue_roll_2 (`KismetMathLibrary.BreakRotator` (`SceneComponent.K2_GetComponentRotation` (`self.Cannon1_Cannon_barrel_002`))))
  (bind _returnvalue (- _returnvalue_roll_2 _startingrotation_roll))
  (bind _returnvalue_2 (- _returnvalue_yaw _startingrotation_yaw))
  (bind _returnvalue_3 (+ _returnvalue (`local.TurnYValue`)))
  (bind _returnvalue_4 (+ _returnvalue_2 (`local.TurnXValue`)))
  ;[1 1 1] Set orientation for turning
  (set `local.TurnXValue` TurnX)
  (bind _result (`/Engine/EditorBlueprintResources/StandardMacros.NegateFloat` TurnY)
    (:`  `
      (set `local.TurnYValue` _result)
      (if (not (>= _returnvalue_4 -55.0))
        (set `local.TurnXValue` (- -55.0 _returnvalue_2)))
      (if (not (<= _returnvalue_4 55.0))
        (set `local.TurnXValue` (- 55.0 _returnvalue_2)))
      ;[1 1 1] Apply final horizontal rotation
      (if true
        (`SceneComponent.K2_AddLocalRotation` (`self.DefaultSceneRoot`) (`KismetMathLibrary.MakeRotator` 0.0 0.0 (`local.TurnXValue`)) false false)
        (if (not (>= _returnvalue_3 -20.0))
          (set `local.TurnYValue` (- -20.0 _returnvalue)))
        (if (not (<= _returnvalue_3 20.0))
          (set `local.TurnYValue` (- 20.0 _returnvalue)))
        ;[1 1 1] Apply final vertical rotation
        (if true
          (`SceneComponent.K2_AddLocalRotation` (`self.Cannon1_Cannon_barrel_002`) (`KismetMathLibrary.MakeRotator` (`local.TurnYValue`)) false false))))))

(fn `UserConstructionScript`)