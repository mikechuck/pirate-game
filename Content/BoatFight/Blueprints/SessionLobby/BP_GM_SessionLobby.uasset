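; Game mode for the session lobby that tracks connected players and launches the match.
; On login it records each player's ID, controller, name and net ID in the GameState list and on their PlayerController; logout removes the entry.
; Both changes fire the GameState's player-list update event.
; StartGame copies the list to GlobalGameInstance, seamless-travels to the gameplay level, and calls each controller's OnStartGame for loading screens.
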(event `self.K2_PostLogin`
  (params (NewPlayer :type "PlayerController Object Reference"))
  (bind _playerstate (`Controller.PlayerState` NewPlayer))
  ;[1 1 1] Initiate new PlayerInfo object for newly connected player
  (bind _asbp_gs_session_lobby (cast `/Game/BoatFight/Blueprints/SessionLobby/BP_GS_SessionLobby` (`GameplayStatics.GetGameState`)))
  (bind _s_playerinfo (make `/Game/BoatFight/Data/S_PlayerInfo` (`/Game/BoatFight/Blueprints/SessionLobby/BP_GS_SessionLobby.NextPlayerId` _asbp_gs_session_lobby) NewPlayer (`KismetTextLibrary.Conv_StringToText` (`PlayerState.GetPlayerName` _playerstate)) false null (struct :`TeamColor` (struct)) (`AdvancedSessionsLibrary.GetUniqueNetIDFromPlayerState` _playerstate)))
  (`KismetArrayLibrary.Array_Add` (`/Game/BoatFight/Blueprints/SessionLobby/BP_GS_SessionLobby.ConnectedPlayerInfo` _asbp_gs_session_lobby) _s_playerinfo)
  ;[1 1 1] Set the player's PC's info
  (bind _asbp_pc_session_lobby (cast `/Game/BoatFight/Blueprints/SessionLobby/BP_PC_SessionLobby` NewPlayer))
  (set `/Game/BoatFight/Blueprints/SessionLobby/BP_PC_SessionLobby.PlayerInfoPC` _s_playerinfo _asbp_pc_session_lobby)
  ;[1 1 1] Increment playerid for the next player that joins
  (bind _asbp_gs_session_lobby_2 (cast `/Game/BoatFight/Blueprints/SessionLobby/BP_GS_SessionLobby` (`GameplayStatics.GetGameState`)))
  (bind _result (`/Engine/EditorBlueprintResources/StandardMacros.IncrementInt` (`/Game/BoatFight/Blueprints/SessionLobby/BP_GS_SessionLobby.NextPlayerId` _asbp_gs_session_lobby_2))
    (:`  `
      (set `/Game/BoatFight/Blueprints/SessionLobby/BP_GS_SessionLobby.NextPlayerId` _result _asbp_gs_session_lobby_2)
      (`self.Emit Player List Update Event`))))

(event `self.K2_OnLogout`
  (params (ExitingController :type "Controller Object Reference"))
  (bind _asplayer_controller (cast `PlayerController` ExitingController))
  (bind _asbp_gs_session_lobby (cast `/Game/BoatFight/Blueprints/SessionLobby/BP_GS_SessionLobby` (`GameplayStatics.GetGameState`)))
  (bind _connectedplayerinfo (`/Game/BoatFight/Blueprints/SessionLobby/BP_GS_SessionLobby.ConnectedPlayerInfo` _asbp_gs_session_lobby))
  ;[1 1 1] Remove leaving player from ConnectedPlayersInfo list
  (for (_array_element _array_index) _connectedplayerinfo
    (if (== (`.PlayerController_4_3BAE9A7943BD0E25B23D19B98BA90CC4` (break `/Game/BoatFight/Data/S_PlayerInfo` _array_element)) _asplayer_controller)
      (`KismetArrayLibrary.Array_Remove` _connectedplayerinfo _array_index)))
  (`self.Emit Player List Update Event`))

(fn `Emit Player List Update Event`
  (`/Game/BoatFight/Blueprints/SessionLobby/BP_GS_SessionLobby.ConnectedPlayersInfoUpdateEvent` (cast `/Game/BoatFight/Blueprints/SessionLobby/BP_GS_SessionLobby` (`GameplayStatics.GetGameState`) :!pure true)))

(fn `StartGame`
  ;[1 1 1] Before server travel, save all info to Game Instance to be used in gameplay level
  (set `/Game/BoatFight/Blueprints/GlobalGameInstance.ConnectedPlayerInfo` (`/Game/BoatFight/Blueprints/SessionLobby/BP_GS_SessionLobby.ConnectedPlayerInfo` (cast `/Game/BoatFight/Blueprints/SessionLobby/BP_GS_SessionLobby` (`GameplayStatics.GetGameState`) :!pure true)) (cast `/Game/BoatFight/Blueprints/GlobalGameInstance` (`GameplayStatics.GetGameInstance`) :!pure true))
  (set `self.bUseSeamlessTravel` true)
  (`AdvancedSessionsLibrary.ServerTravel` "Gameplay_Level_New")
  ;[1 1 1] On StartGame, go through all players all call the OnStartGame client event to trigger loading screen
  (for _array_element (`/Game/BoatFight/Blueprints/SessionLobby/BP_GS_SessionLobby.ConnectedPlayerInfo` (cast `/Game/BoatFight/Blueprints/SessionLobby/BP_GS_SessionLobby` (`GameplayStatics.GetGameState`) :!pure true))
    (bind _asbp_pc_session_lobby (cast `/Game/BoatFight/Blueprints/SessionLobby/BP_PC_SessionLobby` (`.PlayerController_4_3BAE9A7943BD0E25B23D19B98BA90CC4` (break `/Game/BoatFight/Data/S_PlayerInfo` _array_element))))
    (`/Game/BoatFight/Blueprints/SessionLobby/BP_PC_SessionLobby.OnStartGame` _asbp_pc_session_lobby)))

(fn `UserConstructionScript`)