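; Player controller for the session lobby that handles toggling a player's ready status on the server.
; ToggleReadyStatusOnServer finds the entry whose PlayerId matches the given index in GS_SessionLobby's ConnectedPlayerInfo array and rewrites it with IsReady inverted.
; It then has GM_SessionLobby emit a player list update event to notify clients of the change.
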(event `ToggleReadyStatusOnServer`
  (params (PlayerIndex :type Integer))
  (bind _connectedplayerinfo (`/Game/BoatFight/Blueprints/SessionLobby/GS_SessionLobby.ConnectedPlayerInfo` (cast `/Game/BoatFight/Blueprints/SessionLobby/GS_SessionLobby` (`GameplayStatics.GetGameState`) :!pure true)))
  (set `self.ServerRpcPlayerIndex` PlayerIndex)
  ;[1 1 1] Set new Ready value for this player's PlayerInfo record
  (for (_array_element _array_index) _connectedplayerinfo
    (bind (_playerid _playercontroller _playername _isready _playerstate) (break `/Game/BoatFight/Blueprints/SessionLobby/S_PlayerInfo` _array_element))
    (if (== (`self.ServerRpcPlayerIndex`) _playerid)
      (`KismetArrayLibrary.Array_Set` _connectedplayerinfo _array_index (make `/Game/BoatFight/Blueprints/SessionLobby/S_PlayerInfo` _playerid _playercontroller _playername (not _isready) _playerstate))
      ;[1 1 1] Tell GM to emit event to notify all other clients
      (bind _asgm_session_lobby (cast `/Game/BoatFight/Blueprints/SessionLobby/GM_SessionLobby` (`GameplayStatics.GetGameMode`)))
      (`/Game/BoatFight/Blueprints/SessionLobby/GM_SessionLobby.EmitPlayerListUpdateEvent` _asgm_session_lobby))))

(fn `UserConstructionScript`)