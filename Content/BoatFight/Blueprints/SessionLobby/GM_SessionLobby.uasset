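; GM_SessionLobby is the game mode for the session lobby, keeping track of which players are connected.
; On post-login it adds the new player controller to the ConnectedPlayers array on GS_SessionLobby and fires the PlayerListUpdated dispatcher.
; On logout it removes the exiting controller from that array without firing the update.
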(event `self.K2_PostLogin`
  (params (NewPlayer :type "PlayerController Object Reference"))
  (bind _asgs_session_lobby (cast `/Game/BoatFight/Blueprints/SessionLobby/GS_SessionLobby` (`GameplayStatics.GetGameState`)))
  (`KismetArrayLibrary.Array_Add` (`/Game/BoatFight/Blueprints/SessionLobby/GS_SessionLobby.ConnectedPlayers` _asgs_session_lobby) NewPlayer)
  (`self.PlayerListUpdated`))

(event `self.K2_OnLogout`
  (params (ExitingController :type "Controller Object Reference"))
  (bind _asplayer_controller (cast `PlayerController` ExitingController))
  (bind _asgs_session_lobby (cast `/Game/BoatFight/Blueprints/SessionLobby/GS_SessionLobby` (`GameplayStatics.GetGameState`)))
  (`KismetArrayLibrary.Array_RemoveItem` (`/Game/BoatFight/Blueprints/SessionLobby/GS_SessionLobby.ConnectedPlayers` _asgs_session_lobby) _asplayer_controller))

(fn `UserConstructionScript`)