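; Player controller for the session lobby that handles ready toggling, team selection and the start-game transition.
; Server-side events find the player's record by ID in the GameState's ConnectedPlayerInfo, rebuild it, then have the lobby GameMode broadcast a player-list update.
; The team change leaves NetId unset when rebuilding the record, unlike the ready toggle.
; On game start, it shows the HUD loading screen and disables input.
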(event `ToggleReadyStatusOnServer`
  (params (PlayerIndex :type Integer))
  (bind _connectedplayerinfo (`/Game/BoatFight/Blueprints/SessionLobby/BP_GS_SessionLobby.ConnectedPlayerInfo` (cast `/Game/BoatFight/Blueprints/SessionLobby/BP_GS_SessionLobby` (`GameplayStatics.GetGameState`) :!pure true)))
  (set `self.ServerRpcPlayerIndex` PlayerIndex)
  ;[1 1 1] Set new Ready value for this player's PlayerInfo record
  (for (_array_element _array_index) _connectedplayerinfo
    (bind (_playerid _playercontroller _playername _isready _playerstate _team _netid) (break `/Game/BoatFight/Data/S_PlayerInfo` _array_element))
    (if (== (`self.ServerRpcPlayerIndex`) _playerid)
      (`KismetArrayLibrary.Array_Set` _connectedplayerinfo _array_index (make `/Game/BoatFight/Data/S_PlayerInfo` _playerid _playercontroller _playername (not _isready) _playerstate _team _netid))
      ;[1 1 1] Tell GM to emit event to notify all other clients
      (bind _asbp_gm_session_lobby (cast `/Game/BoatFight/Blueprints/SessionLobby/BP_GM_SessionLobby` (`GameplayStatics.GetGameMode`)))
      (`/Game/BoatFight/Blueprints/SessionLobby/BP_GM_SessionLobby.Emit Player List Update Event` _asbp_gm_session_lobby))))

(event `OnStartGame`
  ;[1 1 1] When Start Game is pressed, show loading screen and disable input on the client
  (bind _assession_lobby_hud (cast `/Game/BoatFight/Blueprints/SessionLobby/UI/SessionLobbyHUD` (`self.GetHUD`)))
  (`/Game/BoatFight/Blueprints/SessionLobby/UI/SessionLobbyHUD.ShowLoadingScreen` _assession_lobby_hud)
  (`self.DisableInput` self))

(event `SetTeamOptionOnServer`
  (params (SelectedTeam :type "/Game/BoatFight/Data/S_TeamOption Structure") (PlayerIndex :type Integer))
  (bind _connectedplayerinfo (`/Game/BoatFight/Blueprints/SessionLobby/BP_GS_SessionLobby.ConnectedPlayerInfo` (cast `/Game/BoatFight/Blueprints/SessionLobby/BP_GS_SessionLobby` (`GameplayStatics.GetGameState`) :!pure true)))
  (set `self.SelectedTeamOption` SelectedTeam)
  (set `self.ServerRpcPlayerIndex` PlayerIndex)
  ;[1 1 1] Set new Team value for this player's PlayerInfo record
  (for (_array_element _array_index) _connectedplayerinfo
    (bind (_playerid _playercontroller _playername _isready _playerstate) (break `/Game/BoatFight/Data/S_PlayerInfo` _array_element))
    (if (== (`self.ServerRpcPlayerIndex`) _playerid)
      (`KismetArrayLibrary.Array_Set` _connectedplayerinfo _array_index (make `/Game/BoatFight/Data/S_PlayerInfo` _playerid _playercontroller _playername _isready _playerstate (`self.SelectedTeamOption`)))
      ;[1 1 1] Tell GM to emit event to notify all other clients
      (bind _asbp_gm_session_lobby (cast `/Game/BoatFight/Blueprints/SessionLobby/BP_GM_SessionLobby` (`GameplayStatics.GetGameMode`)))
      (`/Game/BoatFight/Blueprints/SessionLobby/BP_GM_SessionLobby.Emit Player List Update Event` _asbp_gm_session_lobby))))

(fn `UserConstructionScript`)