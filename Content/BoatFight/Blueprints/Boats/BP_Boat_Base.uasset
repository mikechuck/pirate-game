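; BP_Boat_Base is a player-possessable boat pawn base with Enhanced Input controls.
; Possession binds the boat mapping context; look rotates the controller, and move input steps an unclamped index into a speed array.
; Tick pushes the mesh along X with that speed scaled by delta time.
; Interact detaches and repossesses the character, while turning only prints and buoyancy is an empty stub.
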(event `self.ReceiveControllerChanged`
  (params (OldController :type "Controller Object Reference") (NewController :type "Controller Object Reference"))
  (`self.BindControls`))

(event `EnhancedInput|/Game/BoatFight/Inputs/Boat/IA_Boat_Look`
  (params (ActionValue :type "Vector2D Structure") (ElapsedSeconds :type "Float (double-precision)") (TriggeredSeconds :type "Float (double-precision)") (InputAction :type "InputAction Object Reference" :default "/Game/BoatFight/Inputs/Boat/IA_Boat_Look.IA_Boat_Look"))
  ;[0.1961 0.1961 0.1961] Boat Controls
  ;;[1 1 1] Add boat camera controls
  (:`Triggered`
    (`self.AddControllerYawInput` ActionValue_X)
    (`self.AddControllerPitchInput` ActionValue_Y)))

(event `self.ReceiveTick`
  (params (DeltaSeconds :type "Float (single-precision)"))
  (`self.MoveBoat` DeltaSeconds))

(event `EnhancedInput|/Game/BoatFight/Inputs/Boat/IA_Boat_Move`
  (params (ActionValue :type "Vector2D Structure") (ElapsedSeconds :type "Float (double-precision)") (TriggeredSeconds :type "Float (double-precision)") (InputAction :type "InputAction Object Reference" :default "/Game/BoatFight/Inputs/Boat/IA_Boat_Move.IA_Boat_Move"))
  ;[0.1961 0.1961 0.1961] Boat Controls
  ;;[1 1 1] Add boat movement
  (:`Started`
    (`self.ChangeBoatSpeed` ActionValue_Y)))

(event `EnhancedInput|/Game/BoatFight/Inputs/Boat/IA_Boat_Turn`
  (params (ActionValue :type "Vector2D Structure") (ElapsedSeconds :type "Float (double-precision)") (TriggeredSeconds :type "Float (double-precision)") (InputAction :type "InputAction Object Reference" :default "/Game/BoatFight/Inputs/Boat/IA_Boat_Turn.IA_Boat_Turn"))
  ;[0.1961 0.1961 0.1961] Boat Controls
  ;;[1 1 1] Boat turning input
  (:`Triggered`
    (`KismetSystemLibrary.PrintString` "Turning boat")))

(event `EnhancedInput|/Game/BoatFight/Inputs/Boat/IA_Boat_Interact`
  (params (ActionValue :type Boolean) (ElapsedSeconds :type "Float (double-precision)") (TriggeredSeconds :type "Float (double-precision)") (InputAction :type "InputAction Object Reference" :default "/Game/BoatFight/Inputs/Boat/IA_Boat_Interact.IA_Boat_Interact"))
  ;[0.1961 0.1961 0.1961] Boat Controls
  ;;[1 1 1] Boat interaction input
  (:`Triggered`
    (`self.ExitBoat`)))

(fn `ApplyBuoyForce`
  (params (BuoyActor :type "PrimitiveComponent Object Reference") (OtherActor :type "Actor Object Reference")))

(fn `BindControls`
  ;[1 1 1] Add boat mapping context
  (bind _asplayer_controller (cast `PlayerController` (`self.GetController`)))
  (bind _returnvalue (pcsubsystem `EnhancedInputLocalPlayerSubsystem` _asplayer_controller))
  (`EnhancedInputSubsystemInterface.ClearAllMappings` _returnvalue)
  (`EnhancedInputSubsystemInterface.AddMappingContext` _returnvalue "/Game/BoatFight/Inputs/Boat/IMC_Boat.IMC_Boat" 0 (struct)))

(fn `ChangeBoatSpeed`
  (params (MovementInput :type "Float (double-precision)"))
  (set `self.BoatSpeedIndex` (`KismetMathLibrary.FTrunc` (+ MovementInput (`self.BoatSpeedIndex`)))))

(fn `ExitBoat`
  (bind _playercharacterpawn (`self.PlayerCharacterPawn`))
  ;[1 1 1] Detach player from boat
  (`self.K2_DetachFromActor` _playercharacterpawn "KeepWorld" "KeepWorld" "KeepWorld")
  ;[1 1 1] Allow player to move again
  (`self.SetActorEnableCollision` _playercharacterpawn true)
  (`SceneComponent.SetMobility` (`Actor.RootComponent` _playercharacterpawn) "Movable")
  ;[1 1 1] Possess player again
  (bind _asbp_character (cast `/Game/BoatFight/Blueprints/BP_Character` _playercharacterpawn))
  (`Controller.Possess` (`PlayerState.GetPlayerController` (`GameplayStatics.GetPlayerState` 0)) _asbp_character)
  (set `/Game/BoatFight/Blueprints/BP_Character.IsControllingBoat` false _asbp_character))

(fn `MoveBoat`
  (params (DeltaTime :type "Float (double-precision)"))
  (`PrimitiveComponent.AddForce` (`self.StaticMesh`) (`KismetMathLibrary.MakeVector` (* DeltaTime (`|GetArrayItem` (`self.BoatSpeeds`) (`self.BoatSpeedIndex`)))) "None" false))

(fn `UnbindControls`
  ;[1 1 1] Remove player controls
  (`KismetSystemLibrary.PrintString` "Unbinding boat controls" true true (struct :`G` 0.66 :`B` 1.0 :`A` 1.0) 5.0)
  (bind _asplayer_controller (cast `PlayerController` (`self.GetController`)))
  (`EnhancedInputSubsystemInterface.RemoveMappingContext` (pcsubsystem `EnhancedInputLocalPlayerSubsystem` _asplayer_controller) "/Game/BoatFight/Inputs/Boat/IMC_Boat.IMC_Boat" (struct)))

(fn `UserConstructionScript`)