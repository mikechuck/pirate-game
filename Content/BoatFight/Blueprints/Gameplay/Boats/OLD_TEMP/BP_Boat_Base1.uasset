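; Base drivable boat pawn that a player character steers and can exit.
; Enhanced Input handles look and sends throttle-step and rudder changes to the server, with mappings bound on controller change.
; Tick runs movement locally and through a server RPC, applying forward force from a speed array and yaw from rudder divided by speed.
; Exiting detaches the character, with the server repossessing it and multicasting the exit.
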(event `EnhancedInput|/Game/BoatFight/Inputs/Gameplay/Boat/IA_Boat_Look`
  (params (ActionValue :type "Vector2D Structure") (ElapsedSeconds :type "Float (double-precision)") (TriggeredSeconds :type "Float (double-precision)") (InputAction :type "InputAction Object Reference" :default "/Game/BoatFight/Inputs/Gameplay/Boat/IA_Boat_Look.IA_Boat_Look"))
  ;[0.1961 0.1961 0.1961] Boat Controls
  ;;[1 1 1] Add boat camera controls
  (:`Triggered`
    (`self.AddControllerYawInput` ActionValue_X)
    (`self.AddControllerPitchInput` ActionValue_Y)))

(event `EnhancedInput|/Game/BoatFight/Inputs/Gameplay/Boat/IA_Boat_Move`
  (params (ActionValue :type "Vector2D Structure") (ElapsedSeconds :type "Float (double-precision)") (TriggeredSeconds :type "Float (double-precision)") (InputAction :type "InputAction Object Reference" :default "/Game/BoatFight/Inputs/Gameplay/Boat/IA_Boat_Move.IA_Boat_Move"))
  ;[0.1961 0.1961 0.1961] Boat Controls
  ;;[1 1 1] Add boat movement
  (:`Started`
    (`self.SRPC_ChangeBoatSpeed` ActionValue_Y)))

(event `EnhancedInput|/Game/BoatFight/Inputs/Gameplay/Boat/IA_Boat_Turn`
  (params (ActionValue :type "Vector2D Structure") (ElapsedSeconds :type "Float (double-precision)") (TriggeredSeconds :type "Float (double-precision)") (InputAction :type "InputAction Object Reference" :default "/Game/BoatFight/Inputs/Gameplay/Boat/IA_Boat_Turn.IA_Boat_Turn"))
  ;[0.1961 0.1961 0.1961] Boat Controls
  ;;[1 1 1] Boat turning input
  (:`Triggered`
    (`self.SRPC_ChangeRudderAngle` ActionValue_X)))

(event `EnhancedInput|/Game/BoatFight/Inputs/Gameplay/Boat/IA_Boat_Interact`
  (params (ActionValue :type Boolean) (ElapsedSeconds :type "Float (double-precision)") (TriggeredSeconds :type "Float (double-precision)") (InputAction :type "InputAction Object Reference" :default "/Game/BoatFight/Inputs/Gameplay/Boat/IA_Boat_Interact.IA_Boat_Interact"))
  ;[0.1961 0.1961 0.1961] Boat Controls
  ;;[1 1 1] Exit boat
  (:`Triggered`
    (`self.SRPC_ExitBoat` (`GameplayStatics.GetPlayerController` 0))))

(event `self.ReceiveControllerChanged`
  (params (OldController :type "Controller Object Reference") (NewController :type "Controller Object Reference"))
  (`self.CRPC_OnPossessChange` NewController))

(event `CRPC_OnPossessChange`
  (params (NewController :type "Controller Object Reference"))
  ;[0.1036 0.1961 0.08683] Client RPCs
  ;;[1 1 1] Binding controls
  (bind _asplayer_controller (cast `PlayerController` NewController))
  (`self.BindControls` _asplayer_controller))

(event `SRPC_ChangeBoatSpeed`
  (params (MovementInput :type "Float (double-precision)"))
  ;[0.1961 0.09296 0.1067] Server RPCs
  ;;[1 1 1] Change boat speed on input
  (`self.ChangeBoatSpeed` MovementInput))

(event `self.ReceiveTick`
  (params (DeltaSeconds :type "Float (single-precision)"))
  (`self.MoveBoat` DeltaSeconds)
  (`self.SRPC_MoveBoat` DeltaSeconds))

(event `Multicast_ExitBoat`
  (params (OwningPlayerController :type "PlayerController Object Reference"))
  ;[0.1036 0.1961 0.08683] Client RPCs
  ;;[1 1 1] Tell all client to make this player exit the boat
  (`self.ExitBoat` OwningPlayerController))

(event `SRPC_ChangeRudderAngle`
  (params (TurnInput :type "Float (double-precision)"))
  ;[0.1961 0.09296 0.1067] Server RPCs
  ;;[1 1 1] Change rudder angle on input
  (`self.ChangeRudderAngle` TurnInput))

(event `SRPC_ExitBoat`
  (params (PlayerController :type "PlayerController Object Reference") (BoatToExit :type "Actor Object Reference"))
  ;[0.1961 0.09296 0.1067] Server RPCs
  ;;[1 1 1] Exit the boat
  (`self.ExitBoat` PlayerController)
  (`self.Multicast_ExitBoat` PlayerController))

(event `SRPC_MoveBoat`
  (params (DeltaTime :type "Float (double-precision)"))
  ;[0.1961 0.09296 0.1067] Server RPCs
  (`self.MoveBoat` DeltaTime))

(fn `BindControls`
  (params (NewController :type "PlayerController Object Reference"))
  (bind _returnvalue (pcsubsystem `EnhancedInputLocalPlayerSubsystem` NewController))
  ;[1 1 1] Add boat mapping context
  (`/Engine/EditorBlueprintResources/StandardMacros.IsValid` _returnvalue
    (:`Is Valid`
      (`EnhancedInputSubsystemInterface.ClearAllMappings` _returnvalue)
      (`EnhancedInputSubsystemInterface.AddMappingContext` _returnvalue "/Game/BoatFight/Inputs/Gameplay/Boat/IMC_Boat.IMC_Boat" 0 (struct)))))

(fn `ChangeBoatSpeed`
  (params (MovementInput :type "Float (double-precision)"))
  (bind _output_get (set `self.BoatSpeedIndex` (`KismetMathLibrary.Clamp` (`KismetMathLibrary.FTrunc` (+ MovementInput (`self.BoatSpeedIndex`))) 0 3)))
  (`KismetSystemLibrary.PrintString` (`KismetStringLibrary.Concat_StrStr` "Boat Speed Index:" (`KismetStringLibrary.Conv_IntToString` _output_get))))

(fn `ChangeRudderAngle`
  (params (TurnInput :type "Float (double-precision)"))
  (bind _output_get (set `self.RudderAngle` (`KismetMathLibrary.FClamp` (+ (/ TurnInput 10.0) (`self.RudderAngle`)) -1.0)))
  (`KismetSystemLibrary.PrintString` (`KismetStringLibrary.Conv_DoubleToString` _output_get)))

(fn `ExitBoat`
  (params (OwningPlayerController :type "PlayerController Object Reference"))
  (bind _possessingplayerpawn (`self.PossessingPlayerPawn`))
  ;[1 1 1] Detach player from boat
  (`self.K2_DetachFromActor` (`self.PossessingPlayerPawn`) "KeepRelative" "KeepRelative" "KeepRelative")
  ;[1 1 1] Allow player to move again
  (`self.SetActorEnableCollision` _possessingplayerpawn true)
  (`SceneComponent.SetMobility` (`Actor.RootComponent` _possessingplayerpawn) "Movable")
  (if (`KismetSystemLibrary.IsServer`)
    ;[0 0.1961 1] Possess player
    (bind _asbp_character_base (cast `/Game/BoatFight/Blueprints/Gameplay/Players/BP_Character_Base` (`self.PossessingPlayerPawn`)))
    (bind _asbp_pc_gameplay (cast `/Game/BoatFight/Blueprints/Gameplay/BP_PC_Gameplay` (`self.GetOwner`)))
    (`Controller.Possess` _asbp_pc_gameplay _asbp_character_base)
    ;[0 0.1961 1] Set character location so it detaches from boat correctly (replicates to all clients)
    (`SceneComponent.K2_SetWorldLocation` (`Actor.RootComponent` (`self.PossessingPlayerPawn`)) (`SceneComponent.K2_GetComponentLocation` (`self.DriverSocket`)) false false)
    (elif (== (`local.OwningPlayerController`) (`GameplayStatics.GetPlayerController` 0))
      _)))

(fn `MoveBoat`
  (params (DeltaTime :type "Float (double-precision)"))
  (locals (CurrentBoatSpeed :type "Float (double-precision)"))
  (bind _staticmesh (`self.StaticMesh`))
  (bind _output (`|GetArrayItem` (`self.BoatSpeeds`) (`self.BoatSpeedIndex`)))
  (bind (_relativerotation_roll _relativerotation_pitch _relativerotation_yaw) (`KismetMathLibrary.BreakRotator` (`SceneComponent.RelativeRotation` _staticmesh)))
  ;[1 1 1] Apply the correct force for the current selected speed from speed array
  (set `local.CurrentBoatSpeed` _output)
  (`PrimitiveComponent.AddForce` (`self.StaticMesh`) (* (* (* _output (`self.MoveForceMultiplier`)) DeltaTime) (`SceneComponent.GetForwardVector` (`self.StaticMesh`))) "None" true)
  (`SceneComponent.K2_SetRelativeRotation` _staticmesh (`KismetMathLibrary.MakeRotator` 0.0 0.0 (+ _relativerotation_yaw (* (/ (* DeltaTime (`self.RudderAngle`)) (`local.CurrentBoatSpeed`)) 70.0))) false false))

(fn `UnbindControls`
  ;[1 1 1] Remove player controls
  (`KismetSystemLibrary.PrintString` "Unbinding boat controls" true true (struct :`G` 0.66 :`B` 1.0 :`A` 1.0) 5.0)
  (bind _asplayer_controller (cast `PlayerController` (`self.GetController`)))
  (`EnhancedInputSubsystemInterface.RemoveMappingContext` (pcsubsystem `EnhancedInputLocalPlayerSubsystem` _asplayer_controller) "/Game/BoatFight/Inputs/Gameplay/Boat/IMC_Boat.IMC_Boat" (struct)))

(fn `UserConstructionScript`)