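; Gameplay game mode for BoatFight that spawns a Panglang character for each player at a team spawn point and has the player controller possess it.
; It waits until all players saved in GlobalGameInstance log in, then matches them by net ID for team assignment.
; With no saved players, it creates test entries on alternating teams and spawns immediately.
; A looping timer broadcasts a state update event to pace replication.
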(event `self.ReceiveBeginPlay`
  ;[1 1 1] Broadcast "state update event" at an inteval so any replication code knows when to multicast to clients
  (`KismetSystemLibrary.K2_SetTimerDelegate` (delegate `GameStateUpdateEvent`) (`self.StateUpdateInterval`) true))

(event `GameStateUpdateEvent`
  ;[1 1 1] Broadcast "state update event" at an inteval so any replication code knows when to multicast to clients
  (`self.BroadcastStateUpdateEvent`))

(event `self.K2_PostLogin`
  (params (NewPlayer :type "PlayerController Object Reference"))
  (set `self.NewPlayerController` NewPlayer)
  (if (== (`KismetArrayLibrary.Array_Length` (`/Game/BoatFight/Blueprints/GlobalGameInstance.ConnectedPlayerInfo` (cast `/Game/BoatFight/Blueprints/GlobalGameInstance` (`GameplayStatics.GetGameInstance`) :!pure true))) 0)
    (set `self.UseTestData` true)
    ;[1 1 1] Create and spawn test player
    (`self.CreateTestPlayerData` (`self.NewPlayerController`) :!label _label)
    (elif (`self.UseTestData`)
      (goto _label)
      (else
        ;[1 1 1] Use actual connected players
        (`self.CheckPlayersReady`)))))

(fn `BroadcastStateUpdateEvent`
  (`self.StateUpdateEvent`)
  (`/Engine/EditorBlueprintResources/StandardMacros.IncrementInt` (`self.StateUpdateCount`)))

(fn `CheckPlayersReady`
  (bind _result (`/Engine/EditorBlueprintResources/StandardMacros.IncrementInt` (`self.NumPlayersInGame`))
    (:`  `
      (if (== _result (`KismetArrayLibrary.Array_Length` (`/Game/BoatFight/Blueprints/GlobalGameInstance.ConnectedPlayerInfo` (cast `/Game/BoatFight/Blueprints/GlobalGameInstance` (`GameplayStatics.GetGameInstance`) :!pure true))))
        (`self.SpawnAllPlayers`)))))

(fn `CreateTestPlayerData`
  (params (NewPlayerController :type "PlayerController Object Reference"))
  (locals (GameInstance :type "/Game/BoatFight/Blueprints/GlobalGameInstance Object Reference"))
  (bind _output (`|GetArrayItem` (`/Game/BoatFight/Blueprints/GlobalGameInstance.TeamOptions` (`local.GameInstance`)) (`self.TestDateLastAssignedTeam`)))
  (bind _output_get (set `local.GameInstance` (cast `/Game/BoatFight/Blueprints/GlobalGameInstance` (`GameplayStatics.GetGameInstance`) :!pure true)))
  (bind _result (`/Engine/EditorBlueprintResources/StandardMacros.DecrementInt` (`KismetArrayLibrary.Array_Length` (`/Game/BoatFight/Blueprints/GlobalGameInstance.ConnectedPlayerInfo` _output_get)))
    (:`  `
      (switch `int` (`self.TestDateLastAssignedTeam`)
        (:`0`
          (set `self.TestDateLastAssignedTeam` 1))
        (:`1`
          (set `self.TestDateLastAssignedTeam` 0)))
      (`KismetArrayLibrary.Array_Add` (`/Game/BoatFight/Blueprints/GlobalGameInstance.ConnectedPlayerInfo` (`local.GameInstance`)) (make `/Game/BoatFight/Data/S_PlayerInfo` _result NewPlayerController (`KismetTextLibrary.Conv_StringToText` (`KismetStringLibrary.Concat_StrStr` "Test Player " (`KismetStringLibrary.Conv_IntToString` _result))) true (`Controller.PlayerState` NewPlayerController) _output (`AdvancedSessionsLibrary.GetUniqueNetID` NewPlayerController)))
      (`self.SpawnPlayer` NewPlayerController _output))))

(fn `GetSpawnPoint`
  (params (TeamId :type Integer))
  (returns (SpawnPointTransform :type "Transform Structure"))
  (locals (SpawnTag :type String) (SpawnPointLocation :type "Transform Structure"))
  (switch `int` TeamId
    (:`Default`
      (`KismetSystemLibrary.PrintString` "Invalid team ID, can't spawn" true true (struct :`R` 1.0 :`G` 0.019096 :`A` 1.0)))
    (:`0`
      (set `local.SpawnTag` "BlueSpawnPoint")
      (bind _outactors (`GameplayStatics.GetAllActorsWithTag` (`KismetStringLibrary.Conv_StringToName` (`local.SpawnTag`)) :!label _label))
      (for _array_element _outactors
        (bind _asbp_player_spawn (cast `/Game/BoatFight/Blueprints/Gameplay/GameLogic/BP_PlayerSpawn` _array_element)
          (:`then`
            ;[1 1 1] If there are no overlapping actors, spawn is free. Otherwise, wait a second and check again
            (set `local.SpawnPointLocation` (`self.GetTransform` _asbp_player_spawn))
            (if (== (`KismetArrayLibrary.Array_Length` (`PrimitiveComponent.GetOverlappingActors` (`/Game/BoatFight/Blueprints/Gameplay/GameLogic/BP_PlayerSpawn.Box` _asbp_player_spawn) null)) 0)
              (return (`local.SpawnPointLocation`))
              (else
                (`SubmixEffectDelayStatics.SetDelayLength` (make `SubmixEffectDelaySettings` 2000.0) 1.0))))
          (:`CastFailed`
            (`KismetSystemLibrary.PrintString` "Invalid Player Spawn blueprint" true true (struct :`R` 1.0 :`B` 0.007957 :`A` 1.0))))))
    (:`1`
      (set `local.SpawnTag` "RedSpawnPoint")
      (goto _label))))

(fn `SpawnAllPlayers`
  ;[1 1 1] Get all players in the current gamestate base class (added by default)
  (for _array_element (`GameStateBase.PlayerArray` (`GameplayStatics.GetGameState`))
    ;[1 1 1] Loop through players in the gameinstance saved players array
    (for _array_element_2 (`/Game/BoatFight/Blueprints/GlobalGameInstance.ConnectedPlayerInfo` (cast `/Game/BoatFight/Blueprints/GlobalGameInstance` (`GameplayStatics.GetGameInstance`) :!pure true))
      ;[1 1 1] If we match on the net ID, found unique player
      (if (== (`AdvancedSessionsLibrary.GetUniqueNetIDFromPlayerState` _array_element) (`.NetId_28_8D22953142106378BEFAFB9A631EA179` (break `/Game/BoatFight/Data/S_PlayerInfo` _array_element_2)))
        (`self.SpawnPlayer` (`PlayerState.GetPlayerController` _array_element) (`.Team_22_1DF83CF042529DB4A0725AB36210B1BE` (break `/Game/BoatFight/Data/S_PlayerInfo` _array_element_2)))))))

(fn `SpawnPlayer`
  (params (PlayerController :type "PlayerController Object Reference") (PlayerTeam :type "/Game/BoatFight/Data/S_TeamOption Structure"))
  ;[1 1 1] Spawn player pawn and posses by matching player controller
  (bind _spawnpointtransform (`self.GetSpawnPoint` (`.TeamId_2_3A559C5D400BB9A26D863E940CBE7B46` (break `/Game/BoatFight/Data/S_TeamOption` PlayerTeam))))
  (bind _returnvalue (`|SpawnActorFromClass` "/Game/BoatFight/Blueprints/Gameplay/Players/BP_Character_Panglang.BP_Character_Panglang_C" _spawnpointtransform "Undefined" "MultiplyWithRoot" null null))
  (`KismetSystemLibrary.PrintString` "Spawned pawn")
  (`/Game/BoatFight/Blueprints/Gameplay/BP_PC_Gameplay.SRPC_PossessPawn` (cast `/Game/BoatFight/Blueprints/Gameplay/BP_PC_Gameplay` PlayerController :!pure true) _returnvalue)
  (`KismetSystemLibrary.PrintString` "Player possess"))

(fn `UserConstructionScript`)