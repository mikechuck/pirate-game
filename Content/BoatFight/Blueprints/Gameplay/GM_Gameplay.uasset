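; Gameplay game mode for BoatFight that waits for the connected players to log in before spawning a player character.
; PostLogin increments a player count and compares it to the GlobalGameInstance's ConnectedPlayerInfo length, calling SpawnPlayer on a match.
; SpawnPlayer replaces a controller's pawn with a possessed BP_Character_Panglang, but its call passes no controller.
; Debug prints report readiness, and leftover EventGraph test chains are never run.
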(event `self.K2_PostLogin`
  (params (NewPlayer :type "PlayerController Object Reference"))
  (`self.CheckPlayersReady` NewPlayer))

(event `self.ReceiveBeginPlay`)

(event `self.ReceiveTick`
  (params (DeltaSeconds :type "Float (single-precision)")))

(fn `CheckPlayersReady`
  (params (NewPlayerController :type "PlayerController Object Reference"))
  (bind _result (`/Engine/EditorBlueprintResources/StandardMacros.IncrementInt` (`self.NumPlayersInGame`))
    (:`  `
      (if (== _result (`KismetArrayLibrary.Array_Length` (`/Game/BoatFight/Blueprints/GlobalGameInstance.ConnectedPlayerInfo` (cast `/Game/BoatFight/Blueprints/GlobalGameInstance` (`GameplayStatics.GetGameInstance`) :!pure true))))
        (`KismetSystemLibrary.PrintString` "All players spawned")
        (`self.SpawnPlayer` null)
        (else
          (`KismetSystemLibrary.PrintString` "All players NOT spawned"))))))

(fn `SpawnPlayer`
  (params (PlayerController :type "PlayerController Object Reference"))
  (bind _returnvalue (`Controller.K2_GetPawn` PlayerController))
  (`/Engine/EditorBlueprintResources/StandardMacros.IsValid` _returnvalue
    (:`Is Valid`
      (`self.K2_DestroyActor` _returnvalue))
    (:`Is Not Valid`
      _))
  (bind _returnvalue_2 (`|SpawnActorFromClass` "/Game/BoatFight/Blueprints/Gameplay/Players/BP_Character_Panglang.BP_Character_Panglang_C" (`KismetMathLibrary.MakeTransform` (0.0 0.0 0.0)) "Undefined" "MultiplyWithRoot" null null))
  (`Controller.Possess` PlayerController _returnvalue_2))

(fn `UserConstructionScript`)