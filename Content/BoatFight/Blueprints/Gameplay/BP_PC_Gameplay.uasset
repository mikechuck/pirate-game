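; Gameplay player controller for BoatFight that switches input to game-only on BeginPlay and drives periodic player state updates.
; A looping timer at StateUpdateInterval fires the StateUpdateEvent broadcast and increments StateUpdateCount on each tick of the timer.
; SRPC_PossessPawn, named as a server RPC, possesses a supplied pawn.
; ServerPlaySound is a placeholder that only prints a debug string referring to a GM event.
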(event `self.ReceiveBeginPlay`
  (`WidgetBlueprintLibrary.SetInputMode_GameOnly` self)
  ;[1 1 1] Update player state every interval time
  (`KismetSystemLibrary.K2_SetTimerDelegate` (delegate `PlayerStateUpdateEvent`) (`self.StateUpdateInterval`) true))

(event `SRPC_PossessPawn`
  (params (NewPawn :type "Pawn Object Reference"))
  (`self.Possess` NewPawn))

(event `PlayerStateUpdateEvent`
  ;[1 1 1] Update player state every interval time
  (`self.BroadcastStateUpdateEvent`))

(fn `BroadcastStateUpdateEvent`
  (`self.StateUpdateEvent`)
  (`/Engine/EditorBlueprintResources/StandardMacros.IncrementInt` (`self.StateUpdateCount`)))

(fn `ServerPlaySound`
  (`KismetSystemLibrary.PrintString` "Playing sound from GM event"))

(fn `UserConstructionScript`)