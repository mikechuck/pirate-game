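; Possessable, networked boat-mounted cannon that a player aims, fires and exits, swapping in its own Enhanced Input mapping on possession.
; Input goes through server RPCs: aiming and exiting are multicast, while firing spawns BP_Cannonball on the server.
; Aiming yaws the root and rolls the barrel, clamping yaw relative to the parent boat and trimming deltas at limits to avoid stutter.
; Exiting detaches the player pawn, restores its collision and repossesses it server-side.
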(event `self.ReceiveBeginPlay`
  (`self.SetInitialRotation`))

(event `EnhancedInput|/Game/BoatFight/Inputs/Gameplay/Cannon/IA_Cannon_Look`
  (params (ActionValue :type "Vector2D Structure") (ElapsedSeconds :type "Float (double-precision)") (TriggeredSeconds :type "Float (double-precision)") (InputAction :type "InputAction Object Reference" :default "/Game/BoatFight/Inputs/Gameplay/Cannon/IA_Cannon_Look.IA_Cannon_Look"))
  ;[1 1 1] Cannon controls
  ;;[1 1 1] Cannon camera input
  (:`Triggered`
    (`self.SRPC_TurnCannon` ActionValue_X ActionValue_Y)))

(event `self.ReceiveControllerChanged`
  (params (OldController :type "Controller Object Reference") (NewController :type "Controller Object Reference"))
  (`self.CRPC_OnPossessChange` NewController))

(event `self.ReceiveTick`
  (params (DeltaSeconds :type "Float (single-precision)")))

(event `EnhancedInput|/Game/BoatFight/Inputs/Gameplay/Cannon/IA_Cannon_Interact`
  (params (ActionValue :type Boolean) (ElapsedSeconds :type "Float (double-precision)") (TriggeredSeconds :type "Float (double-precision)") (InputAction :type "InputAction Object Reference" :default "/Game/BoatFight/Inputs/Gameplay/Cannon/IA_Cannon_Interact.IA_Cannon_Interact"))
  ;[1 1 1] Cannon controls
  ;;[1 1 1] Exit cannon input
  (:`Triggered`
    (`self.SRPC_ExitCannon` null)))

(event `EnhancedInput|/Game/BoatFight/Inputs/Gameplay/Cannon/IA_Cannon_Shoot`
  (params (ActionValue :type Boolean) (ElapsedSeconds :type "Float (double-precision)") (TriggeredSeconds :type "Float (double-precision)") (InputAction :type "InputAction Object Reference" :default "/Game/BoatFight/Inputs/Gameplay/Cannon/IA_Cannon_Shoot.IA_Cannon_Shoot"))
  ;[1 1 1] Cannon controls
  ;;[1 1 1] Shoot cannon input
  (:`Triggered`
    (`self.SRPC_ShootCannon`)))

(event `CRPC_OnPossessChange`
  (params (NewController :type "Controller Object Reference"))
  ;[0.1036 0.1961 0.08683] Client RPCs
  ;;[1 1 1] On possess, bind new controllers to player controller
  (bind _asplayer_controller (cast `PlayerController` NewController))
  (`self.BindControls` _asplayer_controller))

(event `Multicast_TurnCannon`
  (params (ActionValueX :type "Float (double-precision)") (ActionValueY :type "Float (double-precision)"))
  ;[0.07542 0.1278 0.1961] Multicasts (send all networked versions an event)
  ;;[1 1 1] Tell all client to turn cannon
  (`self.TurnCannon` ActionValueX ActionValueY))

(event `SRPC_TurnCannon`
  (params (ActionValueX :type "Float (double-precision)") (ActionValueY :type "Float (double-precision)"))
  ;[0.1961 0.09296 0.1067] Server RPCs
  ;;[1 1 1] Server tell all clients to turn cannon
  (`self.Multicast_TurnCannon` ActionValueX ActionValueY))

(event `Multicast_ExitCannon`
  (params (OwningPlayerController :type "PlayerController Object Reference"))
  ;[0.07542 0.1278 0.1961] Multicasts (send all networked versions an event)
  ;;[1 1 1] Exit cannon
  (`self.ExitCannon` OwningPlayerController))

(event `SRPC_ShootCannon`
  ;[0.1961 0.09296 0.1067] Server RPCs
  ;;[1 1 1] Server tell all clients to shoot cannon
  (`self.ShootCannon`))

(event `SRPC_ExitCannon`
  (params (OwningPlayerController :type "PlayerController Object Reference"))
  ;[0.1961 0.09296 0.1067] Server RPCs
  ;;[1 1 1] Server exit the boat, then broadcast clients to exit
  (`self.Multicast_ExitCannon` OwningPlayerController))

(fn `BindControls`
  (params (NewPlayerController :type "PlayerController Object Reference"))
  (bind _returnvalue (pcsubsystem `EnhancedInputLocalPlayerSubsystem` NewPlayerController))
  ;[1 1 1] Add cannon mapping context
  (`/Engine/EditorBlueprintResources/StandardMacros.IsValid` _returnvalue
    (:`Is Valid`
      (`EnhancedInputSubsystemInterface.ClearAllMappings` _returnvalue)
      (`EnhancedInputSubsystemInterface.AddMappingContext` _returnvalue "/Game/BoatFight/Inputs/Gameplay/Cannon/IMC_Cannon.IMC_Cannon" 0 (struct)))))

(fn `ExitCannon`
  (params (OwningPlayerController :type "PlayerController Object Reference"))
  ;[1 1 1] Detach player from boat
  (`self.K2_DetachFromActor` (`self.PossessingPlayerPawn`) "KeepWorld" "KeepWorld" "KeepWorld")
  ;[1 1 1] Allow player to move again
  (`self.SetActorEnableCollision` (`self.PossessingPlayerPawn`) true)
  (if (`KismetSystemLibrary.IsServer`)
    (`KismetSystemLibrary.PrintString` "IsServer")
    ;[0 0.1961 1] Possess player
    (bind _asbp_character_base (cast `/Game/BoatFight/Blueprints/Gameplay/Players/BP_Character_Base` (`self.PossessingPlayerPawn`))
      (:`then`
        (bind _asbp_pc_gameplay (cast `/Game/BoatFight/Blueprints/Gameplay/BP_PC_Gameplay` (`self.GetOwner`)))
        (`Controller.Possess` _asbp_pc_gameplay _asbp_character_base))
      (:`CastFailed`
        (`KismetSystemLibrary.PrintString` "Cast failed")))))

(fn `SetInitialRotation`
  ;[1 1 1] Set the initial position as the difference between boat and cannon at spawn
  (set `self.StartingRotation` (`KismetMathLibrary.NormalizedDeltaRotator` (`SceneComponent.K2_GetComponentRotation` (`self.DefaultSceneRoot`)) (`SceneComponent.K2_GetComponentRotation` (`Actor.RootComponent` (`self.GetParentActor`))))))

(fn `ShootCannon`
  (`KismetSystemLibrary.PrintString` "Shooting cannon")
  ;[1 1 1] Shoot bullet from BulletSpawn component
  (`|SpawnActorFromClass` "/Game/BoatFight/Blueprints/Gameplay/Projectiles/BP_Cannonball.BP_Cannonball_C" (`SceneComponent.K2_GetComponentToWorld` (`self.CannonballSpawn`)) "AlwaysSpawn" "MultiplyWithRoot" null null))

(fn `TurnCannon`
  (params (TurnX :type "Float (double-precision)") (TurnY :type "Float (double-precision)"))
  (locals (TurnXValue :type "Float (double-precision)") (TurnYValue :type "Float (double-precision)"))
  (bind _startingrotation_roll (`KismetMathLibrary.BreakRotator` (`self.StartingRotation`)))
  (bind _returnvalue_roll (`KismetMathLibrary.BreakRotator` (`SceneComponent.K2_GetComponentRotation` (`self.Cannon1_Cannon_barrel_002`))))
  (bind _returnvalue (- _returnvalue_roll _startingrotation_roll))
  (bind _returnvalue_2 (+ _returnvalue (`local.TurnYValue`)))
  (bind (_returnvalue_roll_2 _returnvalue_pitch _returnvalue_yaw) (`KismetMathLibrary.BreakRotator` (`KismetMathLibrary.NormalizedDeltaRotator` (`SceneComponent.K2_GetComponentRotation` (`self.DefaultSceneRoot`)) (`KismetMathLibrary.ComposeRotators` (`self.StartingRotation`) (`SceneComponent.K2_GetComponentRotation` (`Actor.RootComponent` (`self.GetParentActor`)))))))
  (bind _returnvalue_3 (+ _returnvalue_yaw (`local.TurnXValue`)))
  ;[1 1 1] Set orientation for turning
  (set `local.TurnXValue` TurnX)
  (bind _result (`/Engine/EditorBlueprintResources/StandardMacros.NegateFloat` TurnY)
    (:`  `
      (set `local.TurnYValue` _result)
      (if (not (>= _returnvalue_3 -55.0))
        (set `local.TurnXValue` (- -55.0 _returnvalue_yaw)))
      (if (not (<= _returnvalue_3 55.0))
        (set `local.TurnXValue` (- 55.0 _returnvalue_yaw)))
      ;[1 1 1] Apply final horizontal rotation
      (`SceneComponent.K2_AddLocalRotation` (`self.DefaultSceneRoot`) (`KismetMathLibrary.MakeRotator` 0.0 0.0 (`local.TurnXValue`)) false false)
      (if (not (>= _returnvalue_2 -20.0))
        (set `local.TurnYValue` (- -20.0 _returnvalue)))
      (if (not (<= _returnvalue_2 20.0))
        (set `local.TurnYValue` (- 20.0 _returnvalue)))
      ;[1 1 1] Apply final vertical rotation
      (`SceneComponent.K2_AddLocalRotation` (`self.Cannon1_Cannon_barrel_002`) (`KismetMathLibrary.MakeRotator` (`local.TurnYValue`)) false false))))

(fn `UserConstructionScript`)