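; Blunderbuss weapon for BoatFight that fires a single bullet per use, gated by a reload timer.
; Tick advances the timer up to ReloadTime, and it starts full so the first shot is immediate.
; UseWeapon calls the parent, resets the timer, spawns BP_Bullet at BulletSpawn and plays the shot sound through a server-to-multicast RPC.
; An unconnected item-action binding and its debug print remain in the graph.
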(event `self.ReceiveBeginPlay`
  (set `self.ReloadTimeElapsed` (`self.ReloadTime`)))

(event `ItemAction_Event_0`
  (`KismetSystemLibrary.PrintString` "Hello"))

(event `self.ReceiveTick`
  (params (DeltaSeconds :type "Float (single-precision)"))
  (`self.CalculateReload` DeltaSeconds))

(event `SRPC_PlayerSound`
  (params (Sound :type "SoundBase Object Reference") (Location :type "Vector Structure"))
  ;[1 1 1] Sound replication
  (`self.Multicast_PlaySound` Sound Location))

(event `Multicast_PlaySound`
  (params (Sound :type "SoundBase Object Reference") (Location :type "Vector Structure"))
  ;[1 1 1] Sound replication
  (`GameplayStatics.PlaySoundAtLocation` Sound Location (struct) 1.0 1.0 0.0 null null null null))

(fn `CalculateReload`
  (params (DeltaTime :type "Float (double-precision)"))
  (bind _reloadtimeelapsed (`self.ReloadTimeElapsed`))
  (bind _returnvalue (+ DeltaTime _reloadtimeelapsed))
  (if (< _reloadtimeelapsed (`self.ReloadTime`))
    (if (> _returnvalue (`self.ReloadTime`))
      (set `self.ReloadTimeElapsed` (`self.ReloadTime`))
      (else
        (set `self.ReloadTimeElapsed` _returnvalue)))))

(fn `UserConstructionScript`)

(fn `UseWeapon`
  (if (>= (`self.ReloadTimeElapsed`) (`self.ReloadTime`))
    (`parent.UseWeapon`)
    (set `self.ReloadTimeElapsed` 0.0)
    ;[1 1 1] Shoot bullet from BulletSpawn component
    (`|SpawnActorFromClass` "/Game/BoatFight/Blueprints/Gameplay/Projectiles/BP_Bullet.BP_Bullet_C" (`SceneComponent.K2_GetComponentToWorld` (`self.BulletSpawn`)) "AlwaysSpawn" "MultiplyWithRoot" null null)
    ;[1 1 1] Shoot sound
    (bind _output_get (set `self.ShootSoundCue` (`self.ShootSoundCue`)))
    (`self.SRPC_PlayerSound` _output_get (`self.K2_GetActorLocation`))))