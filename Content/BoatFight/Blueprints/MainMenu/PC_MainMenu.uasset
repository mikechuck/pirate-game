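; Main menu player controller for BoatFight, meant to switch between the main, create session and join session screens.
; Event handlers add or remove the create and join session widgets on the viewport.
; The setup that creates the widgets, shows the menu and cursor, and binds those handlers is disconnected from BeginPlay, so it never runs.
; In that setup, the create session click binding also has no handler attached.
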(event `self.ReceiveBeginPlay`)

(event `CreateSessionClicked_Event`
  ;[1 1 1] Create Session clicked
  (`UserWidget.AddToViewport` (`self.UI_CreateSession`) 0))

(event `ExitCreateSession_Event`
  ;[1 1 1] Exit create session. Remove from screen
  (`Widget.RemoveFromParent` (`self.UI_CreateSession`)))

(event `JoinSessionClicked_Event`
  ;[1 1 1] Join Session clicked
  (`UserWidget.AddToViewport` (`self.UI_JoinSession`) 0))

(event `ExitJoinSession_Event`
  ;[1 1 1] Exit join session
  (`Widget.RemoveFromParent` (`self.UI_JoinSession`)))

(fn `UserConstructionScript`)