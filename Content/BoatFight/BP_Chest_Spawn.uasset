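; BP_Chest_Spawn scatters BP_Crate loot across the landscape beneath a box placed above the map.
; On BeginPlay the server loops SpawnLoot up to AmountOfLoot.
; Each call traces downward from random points in the box, retrying until it hits near-flat Landscape, identified by class display name.
; It spawns a crate aligned to the hit normal, leaving debug traces and printouts on.
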(event `self.ReceiveBeginPlay`
  (bind _amountofloot (`self.AmountOfLoot`))
  (`/Engine/EditorBlueprintResources/ActorMacros.Switch Has Authority`
    (:`Authority`
      (bind _counter (`/Engine/EditorBlueprintResources/StandardMacros.Do N` _amountofloot :!label _label)
        (:`Exit`
          (`self.SpawnLoot`)
          (if (not (== _counter _amountofloot))
            (goto _label)))))))

(fn `SpawnLoot`
  (bind _returnvalue (`KismetMathLibrary.RandomPointInBoundingBox` (`SceneComponent.K2_GetComponentLocation` (`self.Box`)) (`KismetMathLibrary.MakeVector` (.x (`BoxComponent.GetUnscaledBoxExtent` (`self.Box`))) (.y (`BoxComponent.GetUnscaledBoxExtent` (`self.Box`))) (.z (`BoxComponent.GetUnscaledBoxExtent` (`self.Box`))))))
  ;[1 1 1] Drawing some rays downward and breaknig out their attributes
  (bind (_outhit _returnvalue_2) (`KismetSystemLibrary.LineTraceSingle` :`Start` _returnvalue :`End` (`KismetMathLibrary.MakeVector` (.x _returnvalue) (.y _returnvalue) -1000000.0) :`TraceChannel` "TraceTypeQuery1" :`DrawDebugType` "ForDuration" :`DrawTime` 10.0 :!label _label))
  (bind (_bblockinghit _binitialoverlap _time _distance _location _impactpoint _normal _impactnormal _physmat _hitactor) (`GameplayStatics.BreakHitResult` _outhit))
  (bind _returnvalue_3 (`KismetSystemLibrary.GetClassDisplayName` (`GameplayStatics.GetObjectClass` _hitactor)))
  ;[1 1 1] Make sure the ray is hitting the landscape - if not, try again - keep going until it reaches amount of crates needed
  (if (`KismetStringLibrary.Contains` _returnvalue_3 "Landscape")
    (if (and (< (`KismetMathLibrary.Abs` (.x _normal)) 0.25) (< (`KismetMathLibrary.Abs` (.y _normal)) 0.25) (< (`KismetMathLibrary.Abs` (.z _normal)) 5.0))
      ;[1 1 1] If ray is hitting landscape, arrange object with the normal of the landscape
      (if _returnvalue_2
        (`KismetSystemLibrary.PrintString` (`KismetStringLibrary.Concat_StrStr` _returnvalue_3 "" (`KismetStringLibrary.Conv_VectorToString` _normal)) true true (struct :`G` 0.66 :`B` 1.0 :`A` 1.0) 10.0)
        ;[1 1 1] spawn object
        (`|SpawnActorFromClass` "/Game/BoatFight/BP_Crate.BP_Crate_C" (`KismetMathLibrary.MakeTransform` _location (`KismetMathLibrary.MakeRotator` (.roll (`KismetMathLibrary.Conv_VectorToRotator` _normal)) (- (.pitch (`KismetMathLibrary.Conv_VectorToRotator` _normal)) 90.0) (.yaw (`KismetMathLibrary.Conv_VectorToRotator` _normal)))) "Undefined" "MultiplyWithRoot" null null))
      (else
        (goto _label)))
    (else
      (goto _label))))

(fn `UserConstructionScript`)